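; Sandwich Blueprint for the bistro cooking gameplay that displays its ingredient icons and drives the holding-sandwich HUD preview.
; AddIngredientImg creates an icon widget from the last entry in Ingredients and adds it to the WrapBox of the IngrWidget component's ingredient list.
; Helper functions set that list's visibility and reveal the player HUD's holding-sandwich image if hidden, finding the HUD through a widget class search.
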(event `self.AddIngredientImg`
  (bind _ingredients (`self.Ingredients`))
  (bind _asbp_ingredient_list (cast `/Game/Blueprint/UMG/PlayerBistro/BP_IngredientList` (`WidgetComponent.GetWidget` (`self.IngrWidget`))))
  (bind _returnvalue (`|CreateWidget` "/Game/Blueprint/UMG/PlayerBistro/BP_IngredientImg.BP_IngredientImg_C"))
  (`UserWidget.AddToViewport` _returnvalue 0)
  (`Image.SetBrushFromTexture` (`/Game/Blueprint/UMG/PlayerBistro/BP_IngredientImg.Image_Ingr` _returnvalue) (`.IngrIcon` (break `IngrData` (`Ingredient.CurIngrData` (`|GetArrayItem` _ingredients (- (`KismetArrayLibrary.Array_Length` _ingredients) 1))))) false)
  (`WrapBox.AddChildToWrapBox` (`/Game/Blueprint/UMG/PlayerBistro/BP_IngredientList.WrapBox` _asbp_ingredient_list) _returnvalue))

(fn `SetIngrWidgetVisibility`
  (params (Visibility :type "ESlateVisibility Enum" :default "Visible"))
  (`Widget.SetVisibility` (`WidgetComponent.GetUserWidgetObject` (`self.IngrWidget`)) Visibility))

(fn `SetPreviewVisibility`
  (bind _foundwidgets (`WidgetBlueprintLibrary.GetAllWidgetsOfClass` "/Game/Blueprint/UMG/PlayerBistro/BP_PlayerBistroHUD.BP_PlayerBistroHUD_C"))
  (bind _image_holdingsandwich (`/Game/Blueprint/UMG/PlayerBistro/BP_PlayerBistroHUD.Image_HoldingSandwich` (`|GetArrayItem` _foundwidgets)))
  (if (`|EnumEquality` (`Widget.GetVisibility` _image_holdingsandwich) "Hidden")
    (`Widget.SetVisibility` _image_holdingsandwich "Visible")))

(fn `UserConstructionScript`)