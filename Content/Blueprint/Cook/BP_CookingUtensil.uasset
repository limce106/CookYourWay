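; Cooking utensil Blueprint that shows the cook progress of the ingredient placed on it through a widget.
; BeginPlay casts the Widget component's user widget to BP_CookRate and caches the reference.
; While IsIngredientOn is true, Tick copies the placed ingredient's CurCookRate into that widget's CookRate.
; The graph only reads the ingredient state and never sets it.
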(event `self.ReceiveBeginPlay`
  (bind _asbp_cook_rate (cast `/Game/Blueprint/UMG/BP_CookRate` (`WidgetComponent.GetUserWidgetObject` (`self.Widget`))))
  (set `self.BP_CookRate` _asbp_cook_rate))

(event `self.ReceiveTick`
  (params (DeltaSeconds :type "Float (single-precision)"))
  (if (`self.IsIngredientOn`)
    (set `/Game/Blueprint/UMG/BP_CookRate.CookRate` (`Ingredient.CurCookRate` (`self.PlacedIngredient`)) (`self.BP_CookRate`))))

(fn `UserConstructionScript`)