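; AI controller for the part-timer NPC in the player's bistro, running the BT_PartTimer behavior tree on the BB_PartTimer blackboard.
; Every Tick it polls the world and writes blackboard flags for uncooked ingredients on the cutting board and completed sandwiches on the table.
; The sandwich flag only updates while some BP_DiningTable has a seated customer, so it keeps its last value otherwise.
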(event `self.ReceiveBeginPlay`
  (`self.UseBlackboard` "/Game/AI/BB_PartTimer.BB_PartTimer")
  (`self.RunBehaviorTree` "/Game/AI/BT_PartTimer.BT_PartTimer"))

(event `self.ReceiveTick`
  (params (DeltaSeconds :type "Float (single-precision)"))
  (`self.Set HasUncookedIngrOnCuttingBoard Value`)
  (`self.Set HasCompletedSandwichOnTable Value`))

(fn `CheckIfPlayerBistroHaveCust`
  (returns (Have :type Boolean))
  (bind _outactors (`GameplayStatics.GetAllActorsOfClass` "/Game/Blueprint/Cook/BP_DiningTable.BP_DiningTable_C"))
  (for _array_element _outactors
    (`/Engine/EditorBlueprintResources/StandardMacros.IsValid` (`DiningTable.SeatedCustomer` _array_element)
      (:`Is Valid`
        (return true))))
  (return false))

(fn `Set HasCompletedSandwichOnTable Value`
  (bind _have (`self.CheckIfPlayerBistroHaveCust`))
  (if _have
    (bind _returnvalue (`self.CheckIfCompleteSandwichOnTable`))
    (`BlackboardComponent.SetValueAsBool` (`AIBlueprintHelperLibrary.GetBlackboard` null) "HasCompletedSandwichOnTable" _returnvalue)))

(fn `Set HasUncookedIngrOnCuttingBoard Value`
  (bind _returnvalue (`self.CheckIfUncookedIngrOnCuttingBoard`))
  (`BlackboardComponent.SetValueAsBool` (`AIBlueprintHelperLibrary.GetBlackboard` null) "HasUncookedIngrOnCuttingBoard" _returnvalue))

(fn `UserConstructionScript`)