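; BP_Customer is a customer NPC that presents its patience, comments, taste reviews and payment through widget components.
; Tick feeds normalized Patience into the patience widget, while dialogue and price widgets start hidden.
; Comment and review events briefly show the dialogue bubble, caching the first comment and pulling score-based reviews from CustomerDataManagerSystem; a random comment-chance roll is left unconnected.
; ShowTotalPaidPrice reveals the total paid and plays the payment animation.
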(event `self.ReceiveBeginPlay`
  (`Widget.SetVisibility` (`WidgetComponent.GetUserWidgetObject` (`self.DialogueWidget`)) "Hidden")
  (`Widget.SetVisibility` (`WidgetComponent.GetUserWidgetObject` (`self.PriceWidget`)) "Hidden"))

(event `self.ReceiveTick`
  (params (DeltaSeconds :type "Float (single-precision)"))
  (bind _asbp_patience (cast `/Game/Blueprint/UMG/PlayerBistro/BP_Patience` (`WidgetComponent.GetUserWidgetObject` (`self.PatienceWidget`))))
  (set `/Game/Blueprint/UMG/PlayerBistro/BP_Patience.PatienceRate` (/ (`self.Patience`) 100.0) _asbp_patience))

(event `self.TrySetComment`
  (bind _returnvalue (`WidgetComponent.GetWidget` (`self.DialogueWidget`)))
  (if (`self.IsComment`)
    (`Widget.SetVisibility` (`WidgetComponent.GetWidget` (`self.DialogueWidget`)) "Visible")
    (`KismetSystemLibrary.Delay` 3.0)
    (`Widget.SetVisibility` (`WidgetComponent.GetWidget` (`self.DialogueWidget`)) "Hidden")
    (else
      (set `self.IsComment` true)
      (bind _asbp_dialogue_bubble (cast `/Game/Blueprint/UMG/PlayerBistro/BP_DialogueBubble` _returnvalue))
      (set `self.Dialogue Bubble` _asbp_dialogue_bubble)
      (`Widget.SetVisibility` _returnvalue "Visible")
      (bind _returnvalue_2 (`self.GetComment`))
      (`TextBlock.SetText` (`/Game/Blueprint/UMG/PlayerBistro/BP_DialogueBubble.TextBlock_Dialogue` (`self.Dialogue Bubble`)) (`KismetTextLibrary.Conv_StringToText` _returnvalue_2))
      (`KismetSystemLibrary.Delay` 3.0)
      (`Widget.SetVisibility` (`WidgetComponent.GetWidget` (`self.DialogueWidget`)) "Hidden"))))

(event `self.SetReviewDialogueText`
  (params (TasteScore :type Integer))
  (bind _returnvalue (`WidgetComponent.GetWidget` (`self.DialogueWidget`)))
  (bind _asbp_dialogue_bubble (cast `/Game/Blueprint/UMG/PlayerBistro/BP_DialogueBubble` _returnvalue))
  (set `self.Dialogue Bubble` _asbp_dialogue_bubble)
  (`Widget.SetVisibility` _returnvalue "Visible")
  (bind _returnvalue_2 (`CustomerDataManagerSystem.GetCustReviewDialogue` (subsystem `CustomerDataManagerSystem`) (`self.CustName`) TasteScore))
  (`TextBlock.SetText` (`/Game/Blueprint/UMG/PlayerBistro/BP_DialogueBubble.TextBlock_Dialogue` (`self.Dialogue Bubble`)) (`KismetTextLibrary.Conv_StringToText` _returnvalue_2))
  (`KismetSystemLibrary.Delay` 3.0)
  (`Widget.SetVisibility` (`WidgetComponent.GetWidget` (`self.DialogueWidget`)) "Hidden"))

(fn `ShowTotalPaidPrice`
  (bind _returnvalue (`WidgetComponent.GetUserWidgetObject` (`self.PriceWidget`)))
  (`Widget.SetVisibility` _returnvalue "Visible")
  (bind _asbp_paid_price (cast `/Game/Blueprint/UMG/PlayerBistro/BP_PaidPrice` _returnvalue))
  (bind _returnvalue_2 (`self.GetTotalPaidPrice`))
  (`TextBlock.SetText` (`/Game/Blueprint/UMG/PlayerBistro/BP_PaidPrice.TextBlock_PaidPrcie` _asbp_paid_price) (`KismetTextLibrary.Conv_StringToText` (`KismetStringLibrary.Concat_StrStr` "$ " (`KismetStringLibrary.Conv_IntToString` _returnvalue_2))))
  (`UserWidget.PlayAnimation` _asbp_paid_price (`/Game/Blueprint/UMG/PlayerBistro/BP_PaidPrice.PayPrice_Anim` _asbp_paid_price) 0.0 1 "Forward" 1.0 false))

(fn `UserConstructionScript`)